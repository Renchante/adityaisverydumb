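; Player character with mouse look, movement, double jump, wall running and a first/third-person toggle via spring arm length.
; While falling, Tick traces sideways for "wall"-tagged actors, then aligns yaw to the wall, forces forward velocity, disables gravity and constrains movement to a horizontal plane.
; Jumping off a wall launches away and briefly suspends wall sticking.
; Grounded jumps stack max walk speed for momentum, reset by a retriggerable delay after release.
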(event `InputAction|Jump`
  (params (Key :type "Key Structure"))
  ;[1 1 1] double jump
  (:`Pressed`
    (`/Engine/EditorBlueprintResources/StandardMacros.Do N` 2 :!label _label
      (:`Exit`
        (`self.LaunchCharacter` (`KismetMathLibrary.MakeVector` 0.0 0.0 (`CharacterMovementComponent.JumpZVelocity` (`self.CharacterMovement`))) false true)))))

(event `InputAxis|LookUp`
  (params (AxisValue :type "Float (single-precision)"))
  ;[1 0 0.3055] Mouse Control
  (`self.AddControllerPitchInput` AxisValue))

(event `InputAction|Change Perspective`
  (params (Key :type "Key Structure"))
  (bind _springarm (`self.SpringArm`))
  ;[1 1 1] First to Third Person Toggle
  (:`Pressed`
    (if (== (`SpringArmComponent.TargetArmLength` (`self.SpringArm`)) 1000.0)
      (set `SpringArmComponent.TargetArmLength` 0.0 _springarm)
      (else
        (set `SpringArmComponent.TargetArmLength` 1000.0 _springarm)))))

(event `self.OnLanded`
  (params (Hit :type "HitResult Structure (by ref)"))
  ;[1 1 1] double jump
  (goto _label :!via `Reset`))

(event `InputAxis|Turn`
  (params (AxisValue :type "Float (single-precision)"))
  ;[1 0 0.3055] Mouse Control
  (`self.AddControllerYawInput` AxisValue))

(event `InputAxis|MoveForward`
  (params (AxisValue :type "Float (single-precision)"))
  ;[1 1 1] Comment
  (`self.AddMovementInput` (`self.GetActorForwardVector`) AxisValue))

(event `InputAxis|MoveRight`
  (params (AxisValue :type "Float (single-precision)"))
  ;[1 1 1] Comment
  (`self.AddMovementInput` (`self.GetActorRightVector`) AxisValue))

(event `self.ReceiveBeginPlay`
  (`MovementComponent.SetPlaneConstraintEnabled` (`self.CharacterMovement`) true))

(event `offwall`
  (bind _charactermovement (`self.CharacterMovement`))
  ;[1 1 1] when off the wall
  (set `CharacterMovementComponent.GravityScale` 1.0 _charactermovement)
  (`MovementComponent.SetPlaneConstraintNormal` _charactermovement (0.0 0.0 0.0)))

(event `self.ReceiveTick`
  (params (DeltaSeconds :type "Float (single-precision)"))
  (bind _returnvalue (`self.K2_GetActorLocation`))
  (bind _returnvalue_2 (`self.K2_GetActorLocation`))
  (bind _charactermovement (`self.CharacterMovement`))
  (bind _charactermovement_2 (`self.CharacterMovement`))
  (bind (_returnvalue_x _returnvalue_y) (`KismetMathLibrary.BreakVector` (* (`self.GetActorForwardVector`) 500.0)))
  (bind (_returnvalue_x_2 _returnvalue_y_2) (`KismetMathLibrary.BreakVector` (* (`self.GetActorForwardVector`) 500.0)))
  (if (`NavMovementComponent.IsFalling` (`self.CharacterMovement`))
    (`|ExecutionSequence`
      (:`then_0`
        (if (not (`self.leftside`))
          ;[1 1 1] run on right side of wall
          (bind (_outhit _returnvalue_3) (`KismetSystemLibrary.LineTraceSingle` :`Start` _returnvalue_2 :`End` (+ _returnvalue_2 (* (`self.GetActorRightVector`) 50.0)) :`TraceChannel` "TraceTypeQuery1" :`DrawDebugType` "ForDuration"))
          (bind (_bblockinghit _binitialoverlap _time _distance _location _impactpoint _normal _impactnormal _physmat _hitactor) (`GameplayStatics.BreakHitResult` _outhit))
          (if (and _returnvalue_3 (`self.ActorHasTag` _hitactor "wall"))
            (set `self.rightside` true)
            (set `self.onrightside` true)
            (if (not (`self.isjumpingofwall`))
              (bind (_returnvalue_roll _returnvalue_pitch _returnvalue_yaw) (`KismetMathLibrary.BreakRotator` (`KismetMathLibrary.Conv_VectorToRotator` _normal)))
              (`self.K2_SetActorRotation` (`KismetMathLibrary.MakeRotator` 0.0 0.0 (+ _returnvalue_yaw 90.0)))
              (set `MovementComponent.Velocity` (`KismetMathLibrary.MakeVector` _returnvalue_x_2 _returnvalue_y_2) _charactermovement)
              (set `CharacterMovementComponent.GravityScale` 0.0 _charactermovement)
              (`MovementComponent.SetPlaneConstraintNormal` _charactermovement (0.0 0.0 1.0)))
            (else
              (set `self.rightside` false)
              (`self.offwall`)))))
      (:`then_1`
        (if (not (`self.rightside`))
          ;[1 1 1] run on left side of wall
          (bind (_outhit_2 _returnvalue_4) (`KismetSystemLibrary.LineTraceSingle` _returnvalue (+ _returnvalue (* (`self.GetActorRightVector`) -50.0)) "TraceTypeQuery1"))
          (bind (_bblockinghit_2 _binitialoverlap_2 _time_2 _distance_2 _location_2 _impactpoint_2 _normal_2 _impactnormal_2 _physmat_2 _hitactor_2) (`GameplayStatics.BreakHitResult` _outhit_2))
          (if (and _returnvalue_4 (`self.ActorHasTag` _hitactor_2 "wall"))
            (set `self.leftside` true)
            (set `self.onrightside` false)
            (if (not (`self.isjumpingofwall`))
              (bind (_returnvalue_roll_2 _returnvalue_pitch_2 _returnvalue_yaw_2) (`KismetMathLibrary.BreakRotator` (`KismetMathLibrary.Conv_VectorToRotator` _normal_2)))
              (`self.K2_SetActorRotation` (`KismetMathLibrary.MakeRotator` 0.0 0.0 (+ _returnvalue_yaw_2 -90.0)))
              (set `MovementComponent.Velocity` (`KismetMathLibrary.MakeVector` _returnvalue_x _returnvalue_y) _charactermovement_2)
              (set `CharacterMovementComponent.GravityScale` 0.0 _charactermovement_2)
              (`MovementComponent.SetPlaneConstraintNormal` _charactermovement_2 (0.0 0.0 1.0)))
            (else
              (set `self.leftside` false)
              (`self.offwall`))))))))

(event `InputAction|Jump`
  (params (Key :type "Key Structure"))
  (bind _charactermovement (`self.CharacterMovement`))
  (bind (_returnvalue_x _returnvalue_y) (`KismetMathLibrary.BreakVector` (select `bool` (`self.onrightside`) :`false` (* (`self.GetActorRightVector`) 450.0) :`true` (* (`self.GetActorRightVector`) -450.0))))
  ;[1 1 1] junmping with momentum + wall running
  (:`Pressed`
    (if (or (`self.rightside`) (`self.leftside`))
      (set `self.isjumpingofwall` true)
      (`self.LaunchCharacter` (`KismetMathLibrary.MakeVector` _returnvalue_x _returnvalue_y 450.0))
      (`KismetSystemLibrary.Delay` 0.2)
      (set `self.isjumpingofwall` false)
      (elif (not (`NavMovementComponent.IsFalling` (`self.CharacterMovement`)))
        (`self.Jump`)
        (set `CharacterMovementComponent.MaxWalkSpeed` (`KismetMathLibrary.FClamp` (+ (`MovementComponent.GetMaxSpeed` (`self.CharacterMovement`)) 30.0) 0.0 99999.0) _charactermovement))))
  (:`Released`
    (`KismetSystemLibrary.RetriggerableDelay` 0.8)
    (set `CharacterMovementComponent.MaxWalkSpeed` 600.0 _charactermovement)))

(fn `UserConstructionScript`)